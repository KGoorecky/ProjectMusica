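; BP_Technique_Steal is a battle technique that takes money from its Recipient for the player.
; On BeginPlay, after the parent logic, it adds a truncated tenth of the Recipient's MoneyWorth to PC_Battle's Money, leaving MoneyWorth itself untouched.
; It then shows a message naming thief, amount and target on the current unit's battle HUD, taken from GM_Battle, and clears it after a short delay.
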(event `self.ReceiveBeginPlay`
  (bind _returnvalue (`KismetMathLibrary.FTrunc` (* (`/Game/Dynamic/Characters/Battle/BP_UnitBase.MoneyWorth` (`self.Recipient`)) 0.1)))
  ;[0 0 0 0.5] BeginPlay
  (`parent.ReceiveBeginPlay`)
  (bind _aspc_battle (cast `/Game/Dynamic/Controllers/PC_Battle` (`GameplayStatics.GetPlayerController` 0)))
  (set `/Game/Dynamic/Controllers/PC_Battle.Money` (+ (`/Game/Dynamic/Controllers/PC_Battle.Money` _aspc_battle) _returnvalue) _aspc_battle)
  (bind _asgm_battle (cast `/Game/Dynamic/GameMode/GM_Battle` (`GameplayStatics.GetGameMode`)))
  (set `self.MoneyAmountStolen` _returnvalue)
  (bind _current_unit (`/Game/Dynamic/GameMode/GM_Battle.Current Unit` _asgm_battle))
  (bind _unitbattlehud (`/Game/Dynamic/Blueprints/Components/AC_Combat.UnitBattleHUD` (`/Game/Dynamic/Characters/Battle/BP_UnitBase.Combat Component` _current_unit)))
  (`/Game/Dynamic/Widgets/Battle/WBP_UnitBattleHUD.ShowInformation` _unitbattlehud (`|FormatText` "{name} stole {money} zł from {target}." (`/Game/Dynamic/Characters/Battle/BP_UnitBase.Name` _current_unit) (`self.MoneyAmountStolen`) (`/Game/Dynamic/Characters/Battle/BP_UnitBase.Name` (`self.Recipient`))))
  (`KismetSystemLibrary.Delay` 2.5)
  (`/Game/Dynamic/Widgets/Battle/WBP_UnitBattleHUD.ShowInformation` _unitbattlehud ""))

(fn `UserConstructionScript`
  (`parent.UserConstructionScript`))