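; BP_WhiteMagicBase is the base white magic spell, which applies negative damage to its target, in effect a heal.
; On BeginPlay it casts its instigator to BP_UnitBase and asks that unit's CombatComponent for the base magic damage of the spell's class.
; It negates that value and passes it through ApplyDamage to SpellTarget with the configured damage type, reusing the damage pipeline.
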(event `self.ReceiveBeginPlay`
  (`parent.ReceiveBeginPlay`)
  (bind _asbp_unit_base (cast `/Game/Dynamic/Characters/Battle/BP_UnitBase` (`self.GetInstigator`)))
  (bind _magic_base_damage (`/Game/Dynamic/Blueprints/Components/AC_Combat.CalculateMagicBaseDamage` (`/Game/Dynamic/Characters/Battle/BP_UnitBase.Combat Component` _asbp_unit_base) (`GameplayStatics.GetObjectClass` self)))
  (`GameplayStatics.ApplyDamage` (`self.SpellTarget`) (* _magic_base_damage -1.0) null (`self.GetInstigator`) (`self.Damage Type Class`)))

(fn `UserConstructionScript`
  (`parent.UserConstructionScript`))