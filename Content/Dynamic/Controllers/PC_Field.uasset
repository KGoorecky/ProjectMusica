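; PC_Field is the player controller, apparently for field gameplay, that sets up the gameplay HUD on BeginPlay.
; It creates WBP_GameplayHUD, adds it to the viewport and caches references to both the HUD and the BP_FieldPlayerCharacterBase player character.
; It writes the character's name and formatted level into the HUD's protagonist information widget once, with no later refresh in this Blueprint.
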(event `self.ReceiveBeginPlay`
  (bind _protagonistcharacterinformationwidget (`/Game/Dynamic/Widgets/Field/WBP_GameplayHUD.ProtagonistCharacterInformationWidget` (`self.GameplayHUD`)))
  (bind _returnvalue (`|CreateWidget` "/Game/Dynamic/Widgets/Field/WBP_GameplayHUD.WBP_GameplayHUD_C" self))
  (bind _output_get (set `self.GameplayHUD` _returnvalue))
  (`UserWidget.AddToViewport` _output_get 0)
  (bind _asbp_field_player_character_base (cast `/Game/Dynamic/Characters/Field/BP_FieldPlayerCharacterBase` (`GameplayStatics.GetPlayerCharacter` 0)))
  (set `self.PlayerCharacter` _asbp_field_player_character_base)
  (`TextBlock.SetText` (`/Game/Dynamic/Widgets/Field/WBP_PlayerCharacterInformation.CharacterName` _protagonistcharacterinformationwidget) (`/Game/Dynamic/Characters/Field/BP_FieldCharacterBase.Name` (`self.PlayerCharacter`)))
  (`TextBlock.SetText` (`/Game/Dynamic/Widgets/Field/WBP_PlayerCharacterInformation.CharacterLevel` _protagonistcharacterinformationwidget) (`|FormatText` "Lvl {lvl}" (`/Game/Dynamic/Characters/Field/BP_FieldCharacterBase.CharacterLevel` (`self.PlayerCharacter`)))))

(fn `UserConstructionScript`)