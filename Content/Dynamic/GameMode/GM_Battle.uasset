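; Game mode for turn-based JRPG battles that spawns random enemies from the game instance's pool and manages turns, boost and victory.
; Units queue in TurnOrder, and a DoOnce gate runs one turn at a time through each CombatComponent.
; Party turns fill a boost that temporarily switches music to vocals and adds auras.
; Defeating all enemies triggers victory camera, montages and screen, with timer-ticked EXP payout.
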(event `self.ReceiveBeginPlay`
  ;[0 0 0 0.5] BeginPlay
  (`self.SpawnEnemies`)
  (bind _returnvalue (`GameplayStatics.GetActorOfClass` "/Game/Dynamic/Blueprints/BP_Camera_TopDown.BP_Camera_TopDown_C"))
  (bind _output_get (set `self.MainBattleCamera` _returnvalue))
  (`PlayerController.SetViewTargetWithBlend` (`GameplayStatics.GetPlayerController` 0) _output_get 0.0 "VTBlend_Linear" 0.0 false)
  (bind _outactors (`GameplayStatics.GetAllActorsOfClass` "/Game/Dynamic/Characters/Battle/BP_PartyUnitBase.BP_PartyUnitBase_C"))
  (bind _output_get_2 (set `self.PartyUnits` _outactors))
  (bind _outactors_2 (`GameplayStatics.GetAllActorsOfClass` "/Game/Dynamic/Characters/Battle/BP_EnemyUnitBase.BP_EnemyUnitBase_C"))
  (set `self.EnemyUnits` _outactors_2)
  (`KismetSystemLibrary.Delay` 0.2)
  (bind _aspc_battle (cast `/Game/Dynamic/Controllers/PC_Battle` (`GameplayStatics.GetPlayerController` 0)))
  (set `self.Battle HUD` (`/Game/Dynamic/Controllers/PC_Battle.BattleHUD` _aspc_battle))
  (bind _returnvalue_2 (`GameplayStatics.GetActorOfClass` "/Game/Dynamic/Blueprints/BP_BattleMusicPlayer.BP_BattleMusicPlayer_C"))
  (set `self.BattleMusicPlayer` _returnvalue_2)
  (for _array_element (`self.PartyUnits`)
    (`/Game/Dynamic/Widgets/Battle/WBP_BattleHeadsUpDisplay.AddPartyUnitToHUD` (`self.Battle HUD`) _array_element))
  (`self.CalculateEXPReward`)
  (`self.CalculateMoneyReward`))

(event `TurnRequest`
  (params (Unit :type "/Game/Dynamic/Characters/Battle/BP_UnitBase Object Reference"))
  ;[0 0 0 0.5] Turn Request
  (`KismetArrayLibrary.Array_AddUnique` (`self.TurnOrder`) Unit)
  (`self.StartTurn`))

(event `StartTurn`
  (bind _output (`|GetArrayItem` (`self.TurnOrder`)))
  (bind _combat_component (`/Game/Dynamic/Characters/Battle/BP_UnitBase.Combat Component` _output))
  ;[0 0 0 0.5] StartTurn
  (if (not (`self.IsBattleCompleted`))
    (`/Engine/EditorBlueprintResources/StandardMacros.DoOnce` false :!label _label
      (:`Completed`
        (if (`KismetArrayLibrary.Array_IsValidIndex` (`self.TurnOrder`))
          (`/Engine/EditorBlueprintResources/StandardMacros.IsValid` (`AIBlueprintHelperLibrary.GetAIController` _output)
            (:`Is Valid`
              (`/Game/Dynamic/Blueprints/Components/AC_Combat.StartUnitTurn` _combat_component)
              (set `self.Current Unit` _output)
              (add `/Game/Dynamic/Blueprints/Components/AC_Combat.TurnEnded` _combat_component (`|CreateDelegate` :!event `ReadyNextTurn`))
              (`KismetArrayLibrary.Array_Remove` (`self.TurnOrder`)))
            (:`Is Not Valid`
              (`KismetArrayLibrary.Array_Remove` (`self.TurnOrder`))
              (`self.ReadyNextTurn`)))
          (else
            (`self.ReadyNextTurn`)
            (`PlayerController.SetViewTargetWithBlend` (`GameplayStatics.GetPlayerController` 0) (`self.MainBattleCamera`) 0.0 "VTBlend_Linear" 0.0 false)))))))

(event `ReadyNextTurn`
  ;[0 0 0 0.5] StartTurn
  ;;[0 0 0 0.5] Ready Next Turn
  (`|ExecutionSequence`
    (:`then_0`
      (goto _label :!via `Reset`))
    (:`then_1`
      (if (`KismetArrayLibrary.Array_IsValidIndex` (`self.TurnOrder`))
        (if (`KismetMathLibrary.ClassIsChildOf` (`GameplayStatics.GetObjectClass` (`self.Current Unit`)) "/Game/Dynamic/Characters/Battle/BP_PartyUnitBase.BP_PartyUnitBase_C")
          (`self.DeactivateBoost`)
          (`self.FillBoostBar`))
        (`self.StartTurn`)))))

(event `FillBoostBar`
  ;[0 0 0 0.5] FillBoostBar
  (if (not (`self.IsBoostActive`))
    (set `self.BoostAmount` (+ (`self.BoostAmount`) 0.25))
    (`self.UpdateBoostPercent`)
    (if (== (`self.BoostAmount`) 1.0)
      (`self.ActivateBoost`))))

(event `ActivateBoost`
  ;[0 0 0 0.5] ActivateBoost
  (set `self.BoostAmount` 0.0)
  (set `self.IsBoostActive` true)
  (set `self.BoostTurnsLeft` 3)
  (`self.UpdateBoostPercent`)
  (`AudioParameterControllerInterface.SetTriggerParameter` (`/Game/Dynamic/Blueprints/BP_BattleMusicPlayer.MusicPlayerComponent` (`self.BattleMusicPlayer`)) "ChangeMusicToVocal")
  (`GameplayStatics.PlaySound2D` "/Game/Static/Sound/music-switch-sfx.music-switch-sfx" 1.0 1.0 0.0 null null)
  (for _array_element (`self.PartyUnits`)
    (bind _mesh (`Character.Mesh` _array_element))
    (`MeshComponent.SetOverlayMaterial` _mesh "/Game/Dynamic/Materials/MM_Aura.MM_Aura")
    (`PrimitiveComponent.SetCustomDepthStencilValue` _mesh 128)))

(event `DeactivateBoost`
  ;[0 0 0 0.5] DeactivateBoost
  (if (`self.IsBoostActive`)
    (if (<= (`self.BoostTurnsLeft`) 0)
      (set `self.IsBoostActive` false)
      (`AudioParameterControllerInterface.SetTriggerParameter` (`/Game/Dynamic/Blueprints/BP_BattleMusicPlayer.MusicPlayerComponent` (`self.BattleMusicPlayer`)) "ChangeMusicToInstrumental")
      (`GameplayStatics.PlaySound2D` "/Game/Static/Sound/music-switch-sfx.music-switch-sfx" 1.0 1.0 0.0 null null)
      (for _array_element (`self.PartyUnits`)
        (bind _mesh (`Character.Mesh` _array_element))
        (`MeshComponent.SetOverlayMaterial` _mesh null)
        (`PrimitiveComponent.SetCustomDepthStencilValue` _mesh 0))
      (else
        (`/Engine/EditorBlueprintResources/StandardMacros.DecrementInt` (`self.BoostTurnsLeft`))))))

(fn `AwardEXP`
  (bind _exprewardpertick (`self.EXPRewardPerTick`))
  (bind _expreward (`self.EXPReward`))
  (bind _returnvalue (`KismetMathLibrary.SelectInt` _expreward _exprewardpertick (< _expreward _exprewardpertick)))
  (bind _outactors (`GameplayStatics.GetAllActorsOfClass` "/Game/Dynamic/Characters/Battle/BP_PartyUnitBase.BP_PartyUnitBase_C"))
  (for _array_element _outactors
    (`/Game/Dynamic/Blueprints/Components/AC_Combat.RewardXP` (`/Game/Dynamic/Characters/Battle/BP_UnitBase.Combat Component` _array_element) _returnvalue))
  (bind _output_get (set `self.EXPReward` (- (`self.EXPReward`) _returnvalue)))
  (`self.Update_EXP_UI`)
  (if (<= _output_get 0)
    (`KismetSystemLibrary.K2_ClearAndInvalidateTimerHandle` (`self.EXPRewardTimer`))))

(fn `CalculateEXPReward`
  (locals (Loc_EXPCount :type Integer))
  (for _array_element (`self.EnemyUnits`)
    (set `local.Loc_EXPCount` (+ (`local.Loc_EXPCount`) (`/Game/Dynamic/Characters/Battle/BP_UnitBase.EXP_Worth` _array_element))))
  (set `self.EXPReward` (`local.Loc_EXPCount`)))

(fn `CalculateMoneyReward`
  (locals (Loc_MoneyCount :type Integer))
  (for _array_element (`self.EnemyUnits`)
    (set `local.Loc_MoneyCount` (+ (`local.Loc_MoneyCount`) (`/Game/Dynamic/Characters/Battle/BP_UnitBase.MoneyWorth` _array_element))))
  (set `self.MoneyReward` (`KismetMathLibrary.FTrunc` (* (`local.Loc_MoneyCount`) (`KismetMathLibrary.RandomFloatInRange` 0.8 1.2)))))

(fn `InitiateVictory`
  (bind _battlemusicplayer (`self.BattleMusicPlayer`)
    (:`then`
      (`AudioComponent.FadeOut` (`/Game/Dynamic/Blueprints/BP_BattleMusicPlayer.MusicPlayerComponent` _battlemusicplayer) 0.5 0.0 "Linear")
      (bind _returnvalue (`GameplayStatics.SpawnSound2D` "/Game/Dynamic/MetaSound/Music/MSS_VictoryTheme.MSS_VictoryTheme" 1.0 1.0 0.0 null))
      (set `self.VictoryMusic` _returnvalue)
      (bind _returnvalue_2 (`GameplayStatics.GetActorOfClass` "/Game/Dynamic/Blueprints/BP_VictoryCamera.BP_VictoryCamera_C"))
      (`PlayerController.SetViewTargetWithBlend` (`GameplayStatics.GetPlayerController` 0) _returnvalue_2 0.0 "VTBlend_Linear" 0.0 false)
      (for _array_element (`self.PartyUnits`)
        (`Character.PlayAnimMontage` _array_element (`/Game/Dynamic/Characters/Battle/BP_UnitBase.VictoryAnimation` _array_element) 1.0 "None"))
      (set `self.IsBattleCompleted` true)
      (`KismetSystemLibrary.K2_SetTimer` self "ShowVictoryScreen" 3.0))
    (:`else`)))

(fn `RemoveUnitFromBattle`
  (params (Unit :type "/Game/Dynamic/Characters/Battle/BP_UnitBase Object Reference"))
  (bind _asbp_enemy_unit_base (cast `/Game/Dynamic/Characters/Battle/BP_EnemyUnitBase` Unit)
    (:`then`
      (`KismetArrayLibrary.Array_RemoveItem` (`self.EnemyUnits`) _asbp_enemy_unit_base)
      (if (not (`KismetArrayLibrary.Array_IsValidIndex` (`self.EnemyUnits`)))
        (`KismetSystemLibrary.K2_SetTimer` null "InitiateVictory" 2.0)))
    (:`CastFailed`
      (bind _asbp_party_unit_base (cast `/Game/Dynamic/Characters/Battle/BP_PartyUnitBase` Unit))
      (`KismetArrayLibrary.Array_RemoveItem` (`self.PartyUnits`) _asbp_party_unit_base))))

(fn `ShowVictoryScreen`
  (bind _returnvalue (`|CreateWidget` "/Game/Dynamic/Widgets/Battle/WBP_VictoryScreen.WBP_VictoryScreen_C"))
  (`UserWidget.AddToViewport` _returnvalue 0)
  (`Widget.SetRenderOpacity` (`self.Battle HUD`) 0.0)
  (bind _returnvalue_2 (`KismetSystemLibrary.K2_SetTimer` null "AwardEXP" 0.1 true))
  (set `self.EXPRewardTimer` _returnvalue_2)
  (set `self.EXPRewardPerTick` (/ (`self.EXPReward`) 30)))

(fn `SpawnEnemies`
  (locals (Loc_NumberOfEnemies :type Integer :default 0))
  (bind _outactors (`GameplayStatics.GetAllActorsOfClass` "/Game/Dynamic/Blueprints/BP_BattlePosition.BP_BattlePosition_C"))
  (for _array_element _outactors
    (if (`/Game/Dynamic/Blueprints/BP_BattlePosition.IsEnemyPlacement` _array_element)
      (bind _asgi_jrpg (cast `/Game/Dynamic/GI_JRPG` (`GameplayStatics.GetGameInstance`)))
      (set `/Game/Dynamic/Blueprints/BP_BattlePosition.UnitClass` (`KismetArrayLibrary.Array_Random` (`/Game/Dynamic/GI_JRPG.EnemyPool` _asgi_jrpg)) _array_element)
      (`/Game/Dynamic/Blueprints/BP_BattlePosition.SpawnUnit` _array_element)))
  (return))

(fn `UpdateBoostPercent`
  (bind _wbp_boostbar (`/Game/Dynamic/Widgets/Battle/WBP_BattleHeadsUpDisplay.WBP_BoostBar` (`self.Battle HUD`)))
  (bind _imageswitcher (`/Game/Dynamic/Widgets/Battle/WBP_BoostBar.ImageSwitcher` (`/Game/Dynamic/Widgets/Battle/WBP_BattleHeadsUpDisplay.WBP_BoostBar` (`self.Battle HUD`))))
  (bind _boosttext (`/Game/Dynamic/Widgets/Battle/WBP_BoostBar.BoostTEXT` _wbp_boostbar))
  (`ProgressBar.SetPercent` (`/Game/Dynamic/Widgets/Battle/WBP_BoostBar.BoostBAR` _wbp_boostbar) (`self.BoostAmount`))
  (if (`self.IsBoostActive`)
    (`TextBlock.SetText` _boosttext (`|FormatText` "Boost ACTIVE"))
    (`WidgetSwitcher.SetActiveWidgetIndex` _imageswitcher 1)
    (else
      (`TextBlock.SetText` _boosttext (`|FormatText` "Boost {percent}%" (* (`self.BoostAmount`) 100.0)))
      (`WidgetSwitcher.SetActiveWidgetIndex` _imageswitcher 0))))

(fn `UserConstructionScript`)