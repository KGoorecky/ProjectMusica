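; Base Blueprint for battle enemy units, managing a health widget that shows display name, level and health bar.
; On BeginPlay it passes itself to the widget through update messages, and a separate event refreshes the health bar on request.
; Tick rotates the widget to face the player camera.
; A toggle event uses a FlipFlop to alternate visibility, hiding the widget on its first call.
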(event `self.ReceiveBeginPlay`
  (message `/Game/Dynamic/BlueprintInterfaces/BI_UpdateEnemyHealthBarBattle.UpdateDisplayName` (`WidgetComponent.GetWidget` (`self.HealthWidget`)) self)
  (message `/Game/Dynamic/BlueprintInterfaces/BI_UpdateEnemyHealthBarBattle.UpdateDisplayLevel` (`WidgetComponent.GetWidget` (`self.HealthWidget`)) self)
  (message `/Game/Dynamic/BlueprintInterfaces/BI_UpdateEnemyHealthBarBattle.UpdateHealthBar` (`WidgetComponent.GetWidget` (`self.HealthWidget`)) self))

(event `self.ReceiveTick`
  (params (DeltaSeconds :type "Float (single-precision)"))
  (bind _healthwidget (`self.HealthWidget`))
  (`SceneComponent.K2_SetWorldRotation` _healthwidget (`KismetMathLibrary.FindLookAtRotation` (`SceneComponent.K2_GetComponentLocation` _healthwidget) (`SceneComponent.K2_GetComponentLocation` (`PlayerCameraManager.TransformComponent` (`GameplayStatics.GetPlayerCameraManager` 0)))) false false))

(event `self.UpdateEnemyHealthBar`
  (message `/Game/Dynamic/BlueprintInterfaces/BI_UpdateEnemyHealthBarBattle.UpdateHealthBar` (`WidgetComponent.GetWidget` (`self.HealthWidget`)) self))

(event `self.ToggleEnemyHealthBar`
  (`/Engine/EditorBlueprintResources/StandardMacros.FlipFlop`
    (:`A`
      (`SceneComponent.SetVisibility` (`self.HealthWidget`) false false))
    (:`B`
      (`SceneComponent.SetVisibility` (`self.HealthWidget`) true false))))

(fn `UserConstructionScript`
  (`parent.UserConstructionScript`))