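; Base battle unit that tracks HP and SP, derived on BeginPlay from CombatComponent base stats and modifiers.
; Damage plays a hit reaction, passes through CombatComponent resistance, updates HP and spawns a damage number widget.
; At zero HP it plays a death montage, unpossesses its AI controller and leaves GM_Battle.
; It also provides SP spending, weighted-random loot selection from LootTable and empty health bar events for enemy children to override.
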(event `self.ReceiveBeginPlay`
  (bind _combat_component (`self.Combat Component`))
  (bind ((`HP_2_46E86A8A4676B24D11242AADD73696C1` _hp) (`SP_16_A3A6E68A4E2473AB1A6C9B8DB03B1AF4` _sp)) (break `/Game/Dynamic/Data/S_StatTable` (`/Game/Dynamic/Blueprints/Components/AC_Combat.BaseUnitStats` _combat_component)))
  (bind ((`HP_17_46E86A8A4676B24D11242AADD73696C1` _hp_2) (`SP_18_A3A6E68A4E2473AB1A6C9B8DB03B1AF4` _sp_2)) (break `/Game/Dynamic/Data/S_StatModifier` (`/Game/Dynamic/Blueprints/Components/AC_Combat.UnitStatModifier` _combat_component)))
  ;[0 0 0 0.5] BeginPlay
  (bind _output_get (set `self.HP_Max` (* _hp _hp_2)))
  (set `self.HP_Current` _output_get)
  (bind _output_get_2 (set `self.SP_Max` (* _sp _sp_2)))
  (set `self.SP_Current` _output_get_2))

(event `self.ReceiveAnyDamage`
  (params (Damage :type "Float (single-precision)") (DamageType :type "DamageType Object Reference") (InstigatedBy :type "Controller Object Reference") (DamageCauser :type "Actor Object Reference"))
  ;[0 0 0 0.5] AnyDamage
  (`|ExecutionSequence`
    (:`then_0`
      (if (and (> (`self.HP_Current`) 0.0) (> Damage 0.0))
        (bind _hitreactanimation (`self.HitReactAnimation`)
          (:`then`
            (`|PlayMontage` (`self.Mesh`) _hitreactanimation (`self.HitReactPlayRate`)))
          (:`else`))))
    (:`then_1`
      (bind _newdamage (`/Game/Dynamic/Blueprints/Components/AC_Combat.CalculateDamageResistance` (`self.Combat Component`) Damage))
      (set `self.HP_Current` (`KismetMathLibrary.FClamp` (- (`self.HP_Current`) _newdamage) 0.0 (`self.HP_Max`)))
      (`self.UpdateEnemyHealthBar`)
      (`|ExecutionSequence`
        (:`then_0`
          (bind _returnvalue (`|CreateWidget` "/Game/Dynamic/Widgets/Battle/WBP_DamageNumber.WBP_DamageNumber_C" null _newdamage self))
          (`UserWidget.AddToViewport` _returnvalue 0))
        (:`then_1`
          (if (<= (`self.HP_Current`) 0.0)
            (`|PlayMontage` (`self.Mesh`) (`self.DeathAnimation`) (`self.DeathPlayRate`)
              (:`then`
                (`self.ToggleEnemyHealthBar`)
                (`Controller.UnPossess` (`AIBlueprintHelperLibrary.GetAIController` self))
                (bind _asgm_battle (cast `/Game/Dynamic/GameMode/GM_Battle` (`GameplayStatics.GetGameMode`)))
                (`/Game/Dynamic/GameMode/GM_Battle.RemoveUnitFromBattle` _asgm_battle self)))))))))

(event `UpdateEnemyHealthBar`
  ;[0 0 0 0.5] Enemy Health Bar (This is overriden in EnemyChildClass)
)

(event `ToggleEnemyHealthBar`
  ;[0 0 0 0.5] Enemy Health Bar (This is overriden in EnemyChildClass)
)

(fn `ChooseLoot`
  (returns (Item :type "/Game/Dynamic/ItemSystem/BP_ItemBase Class Reference"))
  (locals (Loc_Sum :type "Float (double-precision)") (Loc_RandomValue :type "Float (double-precision)"))
  (bind _loottable (`self.LootTable`))
  (bind _loottable_2 (`self.LootTable`))
  (`|ExecutionSequence`
    (:`then_0`
      (bind _keys (`BlueprintMapLibrary.Map_Keys` _loottable))
      (for _array_element _keys
        (set `local.Loc_Sum` (+ (`local.Loc_Sum`) (`BlueprintMapLibrary.Map_Find` _loottable _array_element)))))
    (:`then_1`
      (set `local.Loc_RandomValue` (`KismetMathLibrary.RandomFloatInRange` 0.0 (`local.Loc_Sum`)))
      (bind _keys_2 (`BlueprintMapLibrary.Map_Keys` _loottable_2))
      (for _array_element_2 _keys_2
        (bind _value (`BlueprintMapLibrary.Map_Find` _loottable_2 _array_element_2))
        (if (< (`local.Loc_RandomValue`) _value)
          (return _array_element_2)
          (else
            (set `local.Loc_RandomValue` (- (`local.Loc_RandomValue`) _value))))))))

(fn `SpendSP`
  (params (SPCost :type "Float (double-precision)"))
  (set `self.SP_Current` (`KismetMathLibrary.FClamp` (- (`self.SP_Current`) SPCost) 0.0 (`self.SP_Max`)))
  (`self.SPSpent`))

(fn `UserConstructionScript`)