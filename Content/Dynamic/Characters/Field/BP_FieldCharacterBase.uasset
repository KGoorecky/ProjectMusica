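; Base Blueprint for field characters that provides a shared hit reaction.
; HitReact ignores repeat calls while a hit is playing, locks movement and plays the hit montage sped up.
; Completion or interruption releases the hit and movement locks, but only completion also clears the attacking flag.
; HitDetect is an empty function, and the construction script does nothing.
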(event `HitReact`
  ;[0 0 0 0.5] Hit React
  (if (not (`self.IsGettingHit`))
    (set `self.IsGettingHit` true)
    (set `self.CanMove` false)
    (`|PlayMontage` (`self.Mesh`) (`self.HitReactMontage`) 1.5
      (:`OnCompleted`
        (set `self.IsAttacking` false))
      (:`OnInterrupted`
        _))
    (set `self.IsGettingHit` false)
    (set `self.CanMove` true)))

(fn `HitDetect`)

(fn `UserConstructionScript`)