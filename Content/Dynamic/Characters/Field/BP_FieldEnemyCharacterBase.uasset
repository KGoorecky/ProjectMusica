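; Base overworld enemy for a JRPG that chases encounters, taking field damage and stun and showing them on a camera-facing info widget.
; Pawn sensing and a deaggro sphere toggle the AI blackboard's HasSeenPlayer and update overworld music.
; A full stun bar or a right-hand sphere-trace hit on the player starts battle, passing EnemyPool to GI_JRPG before a transition into MAP_DebugBattle.
; Depleted health destroys the enemy without a battle.
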(event `/Game/Dynamic/BlueprintInterfaces/BI_ApplyStun.ApplyStun`
  (params (StunCauser :type "/Game/Dynamic/Characters/Field/BP_FieldCharacterBase Object Reference") (`Base Stun` :type "Float (double-precision)"))
  (if (`/Game/Dynamic/Characters/Field/BP_FieldCharacterBase.CanDamageOpponent` StunCauser)
    (bind _output_get (set `self.Current Stun` (+ (`self.Current Stun`) `Base Stun`)))
    (message `/Game/Dynamic/BlueprintInterfaces/BI_UpdateEnemyInfoBarField.UpdateStunBar` (`WidgetComponent.GetWidget` (`self.InfoWidgetComponent`)) self)
    (if (>= _output_get (`self.Max Stun`))
      (`self.StartBattle`))))

(event `self.ReceiveAnyDamage`
  (params (Damage :type "Float (single-precision)") (DamageType :type "DamageType Object Reference") (InstigatedBy :type "Controller Object Reference") (DamageCauser :type "Actor Object Reference"))
  (if (`/Game/Dynamic/Characters/Field/BP_FieldCharacterBase.CanDamageOpponent` (stale `/Game/Dynamic/BlueprintInterfaces/BI_ApplyStun.ApplyStun` StunCauser))
    (set `/Game/Dynamic/Characters/Field/BP_FieldCharacterBase.CanDamageOpponent` false (stale `/Game/Dynamic/BlueprintInterfaces/BI_ApplyStun.ApplyStun` StunCauser))
    (bind _output_get (set `self.Current Health` (- (`self.Current Health`) Damage)))
    (`self.HitReact`)
    (message `/Game/Dynamic/BlueprintInterfaces/BI_UpdateEnemyInfoBarField.UpdateHealthBar` (`WidgetComponent.GetWidget` (`self.InfoWidgetComponent`)) self)
    (if (<= _output_get 0.0)
      (`self.K2_DestroyActor`))))

(event `self.ReceiveBeginPlay`
  (message `/Game/Dynamic/BlueprintInterfaces/BI_UpdateEnemyInfoBarField.UpdateNameDisplay` (`WidgetComponent.GetWidget` (`self.InfoWidgetComponent`)) self)
  (message `/Game/Dynamic/BlueprintInterfaces/BI_UpdateEnemyInfoBarField.UpdateStunBar` (`WidgetComponent.GetWidget` (`self.InfoWidgetComponent`)) self)
  (message `/Game/Dynamic/BlueprintInterfaces/BI_UpdateEnemyInfoBarField.UpdateHealthBar` (`WidgetComponent.GetWidget` (`self.InfoWidgetComponent`)) self)
  (bind _returnvalue (`GameplayStatics.GetActorOfClass` "/Game/Dynamic/Blueprints/BP_OverworldMusicPlayer.BP_OverworldMusicPlayer_C"))
  (set `self.OverworldMusicPlayerRef` _returnvalue))

(event `Attack`
  (if (not (`self.IsGettingHit`))
    (set `self.CanMove` false)
    (`|PlayMontage` (`self.Mesh`) (`self.Attack Montage`)
      (:`OnCompleted`
        _)
      (:`OnInterrupted`
        _))
    (set `self.CanMove` true)
    (set `self.CanAttackDetectHit` true)))

(event `StartBattle`
  (bind _battletransition (`self.BattleTransition`))
  (bind _asgi_jrpg (cast `/Game/Dynamic/GI_JRPG` (`GameplayStatics.GetGameInstance`)))
  (set `/Game/Dynamic/GI_JRPG.EnemyPool` (`self.EnemyPool`) _asgi_jrpg)
  (bind _returnvalue (`|CreateWidget` "/Game/Dynamic/Widgets/Field/WBP_BattleTransition.WBP_BattleTransition_C" (`GameplayStatics.GetPlayerController` 0)))
  (bind _output_get (set `self.BattleTransition` _returnvalue))
  (`UserWidget.AddToViewport` _output_get 0)
  (`|PlayAnimation2` _battletransition (`/Game/Dynamic/Widgets/Field/WBP_BattleTransition.BattleTransitionAnim` _battletransition)
    (:`then`
      (`GameplayStatics.SetGamePaused` true))
    (:`Finished`
      (`GameplayStatics.OpenLevelBySoftObjectPtr` "/Game/Dynamic/Maps/MAP_DebugBattle.MAP_DebugBattle"))))

(event `self.ReceiveTick`
  (params (DeltaSeconds :type "Float (single-precision)"))
  (bind _infowidgetcomponent (`self.InfoWidgetComponent`))
  ;[0 0 0 0.5] Event Tick
  (`SceneComponent.K2_SetWorldRotation` _infowidgetcomponent (`KismetMathLibrary.FindLookAtRotation` (`SceneComponent.K2_GetComponentLocation` _infowidgetcomponent) (`SceneComponent.K2_GetComponentLocation` (`PlayerCameraManager.TransformComponent` (`GameplayStatics.GetPlayerCameraManager` 0)))) false false))

(event `self.PawnSensing.OnSeePawn`
  (params (Pawn :type "Pawn Object Reference"))
  ;[0 0 0 0.5] Detect and Lose Player
  (if (== Pawn (`GameplayStatics.GetPlayerCharacter` 0))
    (`BlackboardComponent.SetValueAsBool` (`AIBlueprintHelperLibrary.GetBlackboard` (`AIBlueprintHelperLibrary.GetAIController` self)) "HasSeenPlayer" true)
    (`/Engine/EditorBlueprintResources/StandardMacros.DoOnce` false :!label _label
      (:`Completed`
        (message `/Game/Dynamic/BlueprintInterfaces/BI_PlayerSpotted.PlaySpottedAnim` (`WidgetComponent.GetWidget` (`self.SpottedWidgetComponent`)))
        (`KismetArrayLibrary.Array_AddUnique` (`/Game/Dynamic/Blueprints/BP_OverworldMusicPlayer.FocusedEnemies` (`self.OverworldMusicPlayerRef`)) self)
        (`/Game/Dynamic/Blueprints/BP_OverworldMusicPlayer.ChangeMusicType` (`self.OverworldMusicPlayerRef`))))))

(event `self.Deaggro Sphere.OnComponentEndOverlap`
  (params (OverlappedComponent :type "PrimitiveComponent Object Reference") (OtherActor :type "Actor Object Reference") (OtherComp :type "PrimitiveComponent Object Reference") (OtherBodyIndex :type Integer))
  ;[0 0 0 0.5] Detect and Lose Player
  (if (== OtherActor (`GameplayStatics.GetPlayerCharacter` 0))
    (`BlackboardComponent.SetValueAsBool` (`AIBlueprintHelperLibrary.GetBlackboard` (`AIBlueprintHelperLibrary.GetAIController` self)) "HasSeenPlayer" false)
    (`KismetArrayLibrary.Array_RemoveItem` (`/Game/Dynamic/Blueprints/BP_OverworldMusicPlayer.FocusedEnemies` (`self.OverworldMusicPlayerRef`)) self)
    (`/Game/Dynamic/Blueprints/BP_OverworldMusicPlayer.ChangeMusicType` (`self.OverworldMusicPlayerRef`))
    (goto _label :!via `Reset`)))

(fn `HitDetect`
  (bind _returnvalue (`SceneComponent.GetSocketLocation` (`self.Mesh`) "RightHand"))
  (if (`self.CanAttackDetectHit`)
    (bind (_outhit _returnvalue_2) (`KismetSystemLibrary.SphereTraceSingleForObjects` :`Start` _returnvalue :`End` (+ _returnvalue (* (`self.GetActorForwardVector`) 64.0)) :`Radius` 48.0 :`ObjectTypes` (`|MakeArray` "ObjectTypeQuery3" :!type "EObjectTypeQuery Enum") :`DrawDebugType` "ForDuration"))
    (if _returnvalue_2
      (if (`KismetMathLibrary.ClassIsChildOf` (`GameplayStatics.GetObjectClass` (`.HitActor` (`GameplayStatics.BreakHitResult` _outhit))) "/Game/Dynamic/Characters/Field/BP_FieldPlayerCharacterBase.BP_FieldPlayerCharacterBase_C")
        (set `self.CanAttackDetectHit` false)
        (`self.StartBattle`)))))

(fn `UserConstructionScript`
  (`parent.UserConstructionScript`))