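; BP_FieldPlayerCharacterBase is the base Blueprint for player characters in field gameplay, providing melee hit detection.
; HitDetect sphere-traces forward from the RightHand socket for Pawn objects, with debug drawing on.
; If the hit actor is a BP_FieldEnemyCharacterBase, it sends ApplyStunMessage and applies damage.
; Stun and damage amounts are selected by AttackCount, so the later combo steps hit harder.
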(fn `HitDetect`
  (bind _returnvalue (`SceneComponent.GetSocketLocation` (`self.Mesh`) "RightHand"))
  (bind (_outhit _returnvalue_2) (`KismetSystemLibrary.SphereTraceSingleForObjects` :`Start` _returnvalue :`End` (+ _returnvalue (* (`self.GetActorForwardVector`) 96.0)) :`Radius` 48.0 :`ObjectTypes` (`|MakeArray` "ObjectTypeQuery3" :!type "EObjectTypeQuery Enum") :`DrawDebugType` "ForDuration"))
  (if _returnvalue_2
    (bind (_bblockinghit _binitialoverlap _time _distance _location _impactpoint _normal _impactnormal _physmat _hitactor) (`GameplayStatics.BreakHitResult` _outhit))
    (if (`KismetMathLibrary.ClassIsChildOf` (`GameplayStatics.GetObjectClass` _hitactor) "/Game/Dynamic/Characters/Field/BP_FieldEnemyCharacterBase.BP_FieldEnemyCharacterBase_C")
      (message `/Game/Dynamic/BlueprintInterfaces/BI_ApplyStun.ApplyStun` _hitactor self (select `int` (- (`self.AttackCount`) 1) :`0` 15.0 :`1` 15.0 :`2` 25.0 :`3` 25.0 :!type "Float (single-precision)"))
      (`GameplayStatics.ApplyDamage` _hitactor (select `int` (- (`self.AttackCount`) 1) :`0` 5.0 :`1` 5.0 :`2` 10.0 :`3` 10.0 :!type "Float (single-precision)") null self))))

(fn `UserConstructionScript`
  (`parent.UserConstructionScript`))