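; BP_NPCBase is the NPC base Blueprint, showing a name and title above the character through an overhead widget component.
; On BeginPlay it casts the component's widget to BP_NPCOverHeadInfo, caches it, and fills in the name and tilde-wrapped title.
; Every Tick it billboards the widget component by rotating it toward the first player's camera manager location.
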(event `self.ReceiveBeginPlay`
  (bind _asbp_npcover_head_info (cast `/Game/Dynamic/Widgets/NPC/BP_NPCOverHeadInfo` (`WidgetComponent.GetWidget` (`self.OverHeadInfoWidgetComponent`))))
  (set `self.NPC_OverHeadInfoWidget` _asbp_npcover_head_info)
  (`TextBlock.SetText` (`/Game/Dynamic/Widgets/NPC/BP_NPCOverHeadInfo.CharacterName` (`self.NPC_OverHeadInfoWidget`)) (`self.CharacterName`))
  (`TextBlock.SetText` (`/Game/Dynamic/Widgets/NPC/BP_NPCOverHeadInfo.CharacterTitle` (`self.NPC_OverHeadInfoWidget`)) (`|FormatText` "~{title}~" (`self.CharacterTitle`))))

(event `self.ReceiveTick`
  (params (DeltaSeconds :type "Float (single-precision)"))
  (bind _overheadinfowidgetcomponent (`self.OverHeadInfoWidgetComponent`))
  (`SceneComponent.K2_SetWorldRotation` _overheadinfowidgetcomponent (`KismetMathLibrary.FindLookAtRotation` (`SceneComponent.K2_GetComponentLocation` _overheadinfowidgetcomponent) (`SceneComponent.K2_GetComponentLocation` (`PlayerCameraManager.TransformComponent` (`GameplayStatics.GetPlayerCameraManager` 0)))) false false))

(fn `UserConstructionScript`)