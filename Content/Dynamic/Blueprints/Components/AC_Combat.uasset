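; AC_Combat is the turn-based combat component on battle units, handling turn timing, actions, damage formulas and XP leveling.
; It loads stats by level from a data table, then runs an agility-scaled timer that requests turns from GM_Battle.
; Party units get a battle HUD; enemies basic-attack a random party member.
; Commands chain AI movement, montages, notify-timed spawns and dynamic camera changes, then return the unit and restart its timer.
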(event `self.ReceiveBeginPlay`
  ;[0 0 0 0.5] Begin Play
  (bind _asbp_unit_base (cast `/Game/Dynamic/Characters/Battle/BP_UnitBase` (`self.GetOwner`)))
  (bind _output_get (set `self.UnitCharacter` _asbp_unit_base))
  (set `self.BattlePosition` (`Actor.GetTransform` _output_get))
  (bind _returnvalue (`|GetDataTableRow` "/Game/Dynamic/Data/DT_BaseStatTable.DT_BaseStatTable" (`KismetStringLibrary.Conv_StringToName` (`KismetStringLibrary.Conv_IntToString` (`self.UnitLevel`))))
    (:`then`
      (set `self.BaseUnitStats` _returnvalue)
      (`self.BeginBattle`))))

(event `UseItemOnEnemy`
  (params (Item :type "/Game/Dynamic/ItemSystem/BP_ItemBase Class Reference"))
  (bind _battleposition_location (`KismetMathLibrary.BreakTransform` (`self.BattlePosition`)))
  (bind _unittarget (`self.UnitTarget`))
  ;[0 0 0 0.5] Items
  ;;[0 0 0 0.5] Use Item On Enemy
  (`|AIMoveTo` (`self.UnitCharacter`) (`self.GetRangePosition` true) null 100.0
    (:`then`
      (`self.RemoveUnitBattleHUD`))
    (:`OnSuccess`
      (`|PlayMontage` (`Character.Mesh` (`self.UnitCharacter`)) (`self.ItemUseMontage`) (`self.ItemUsePlayRate`)
        (:`then`
          (message `/Game/Dynamic/BlueprintInterfaces/BI_DynamicCamera.SetLookAtActor` (`Controller.GetViewTarget` (`GameplayStatics.GetPlayerController` 0)) (`self.UnitTarget`)))
        (:`OnCompleted`
          (`|AIMoveTo` (`self.UnitCharacter`) _battleposition_location null
            (:`OnSuccess`
              (`AIController.K2_SetFocus` (`AIBlueprintHelperLibrary.GetAIController` (`self.UnitCharacter`)) (`self.UnitTarget`))
              (`KismetSystemLibrary.Delay` 1.0)
              (`self.EndUnitTurn`))))
        (:`OnNotifyBegin`
          (`|SpawnActorFromClass` Item (`Actor.GetTransform` _unittarget) "Undefined" "MultiplyWithRoot" null _unittarget (`self.UnitCharacter`)))))))

(event `Attack Command`
  ;[0 0 0 0.5] Attack Command
  (message `/Game/Dynamic/BlueprintInterfaces/BI_DynamicCamera.SetOrbit` (`Controller.GetViewTarget` (`GameplayStatics.GetPlayerController` 0)) false)
  (if (`self.IsRangedCharacter`)
    (`self.RangedAttack`)
    (else
      (`self.Meele Attack`))))

(event `Magic Command`
  (params (`Magic Class` :type "/Game/Dynamic/Abilities/Magic/BP_MagicBase Class Reference"))
  ;[0 0 0 0.5] Magic Command
  (message `/Game/Dynamic/BlueprintInterfaces/BI_DynamicCamera.SetOrbit` (`Controller.GetViewTarget` (`GameplayStatics.GetPlayerController` 0)) false)
  (if (`KismetMathLibrary.ClassIsChildOf` `Magic Class` "/Game/Dynamic/Abilities/Magic/BlackMagic/BP_BlackMagicBase.BP_BlackMagicBase_C")
    (`self.Cast Black Magic` `Magic Class`)
    (else
      (`self.CastWhiteMagic` `Magic Class`))))

(event `Items Command`
  (params (Item :type "/Game/Dynamic/ItemSystem/BP_ItemBase Class Reference"))
  ;[0 0 0 0.5] Item Command
  (message `/Game/Dynamic/BlueprintInterfaces/BI_DynamicCamera.SetOrbit` (`Controller.GetViewTarget` (`GameplayStatics.GetPlayerController` 0)) false)
  (switch `/Game/Dynamic/ItemSystem/ENUM_ItemsType` (`.Type_11_0DF98F624C32CA1D0C9ED08CF68FE168` (break `/Game/Dynamic/ItemSystem/S_ItemDetails` (defaults `Object` Item)))
    (:`NewEnumerator0`
      (`self.UseItemOnAllies` Item :!label _label))
    (:`NewEnumerator6`
      (goto _label))
    (:`NewEnumerator1`
      (goto _label))
    (:`NewEnumerator2`
      (`self.UseItemOnEnemy` Item))))

(event `UseItemOnAllies`
  (params (Item :type "/Game/Dynamic/ItemSystem/BP_ItemBase Class Reference"))
  (bind (_battleposition_location _battleposition_rotation) (`KismetMathLibrary.BreakTransform` (`self.BattlePosition`)))
  (bind _unittarget (`self.UnitTarget`))
  ;[0 0 0 0.5] Items
  ;;[0 0 0 0.5] Use Item On Allies
  (`|AIMoveTo` (`self.UnitCharacter`) (`self.GetRangePosition` false) null 100.0
    (:`then`
      (`self.RemoveUnitBattleHUD`))
    (:`OnSuccess`
      (`|PlayMontage` (`Character.Mesh` (`self.UnitCharacter`)) (`self.ItemUseMontage`) (`self.ItemUsePlayRate`)
        (:`then`
          (message `/Game/Dynamic/BlueprintInterfaces/BI_DynamicCamera.SetLookAtActor` (`Controller.GetViewTarget` (`GameplayStatics.GetPlayerController` 0)) (`self.UnitTarget`))
          (message `/Game/Dynamic/BlueprintInterfaces/BI_DynamicCamera.SetDynamicLocation` (`Controller.GetViewTarget` (`GameplayStatics.GetPlayerController` 0)) (`self.UnitTarget`) (0.0 0.0 0.0)))
        (:`OnCompleted`
          (`|AIMoveTo` (`self.UnitCharacter`) _battleposition_location null
            (:`OnSuccess`
              (`AIController.K2_SetFocalPoint` (`AIBlueprintHelperLibrary.GetAIController` (`self.UnitCharacter`)) (+ _battleposition_location (* (`KismetMathLibrary.GetForwardVector` _battleposition_rotation) 200.0)))
              (`KismetSystemLibrary.Delay` 1.0)
              (`self.EndUnitTurn`))))
        (:`OnNotifyBegin`
          (`|SpawnActorFromClass` Item (`Actor.GetTransform` _unittarget) "Undefined" "MultiplyWithRoot" null _unittarget (`self.UnitCharacter`)))))))

(event `TechniqueCommand`
  (params (Technique :type "/Game/Dynamic/Abilities/Techniques/BP_TechniqueBase Class Reference"))
  ;[0 0 0 0.5] Technique Command
  (message `/Game/Dynamic/BlueprintInterfaces/BI_DynamicCamera.SetOrbit` (`Controller.GetViewTarget` (`GameplayStatics.GetPlayerController` 0)) false)
  (if (`.IsFriendly` (defaults `Object` Technique))
    (`self.UseTechniqueOnAllies` Technique)
    (else
      (`self.UseTechniqueOnEnemy` Technique))))

(event `Meele Attack`
  (bind _battleposition_location (`KismetMathLibrary.BreakTransform` (`self.BattlePosition`)))
  ;[0 0 0 0.5] Basic Attack
  (`|AIMoveTo` (`self.UnitCharacter`) (0.0 0.0 0.0) (`self.UnitTarget`) 100.0
    (:`then`
      (`self.RemoveUnitBattleHUD`))
    (:`OnSuccess`
      (`|PlayMontage` (`Character.Mesh` (`self.UnitCharacter`)) (`self.AttackMontage`) (`self.AttackPlayRate`)
        (:`OnCompleted`
          (`|AIMoveTo` (`self.UnitCharacter`) _battleposition_location null
            (:`then`
              (message `/Game/Dynamic/BlueprintInterfaces/BI_DynamicCamera.SetOrbit` (`Controller.GetViewTarget` (`GameplayStatics.GetPlayerController` 0)) false))
            (:`OnSuccess`
              (`AIController.K2_SetFocus` (`AIBlueprintHelperLibrary.GetAIController` (`self.UnitCharacter`)) (`self.UnitTarget`))
              (`KismetSystemLibrary.Delay` 1.0)
              (`self.EndUnitTurn`))))))))

(event `UseTechniqueOnEnemy`
  (params (Technique :type "/Game/Dynamic/Abilities/Techniques/BP_TechniqueBase Class Reference"))
  (bind _battleposition_location (`KismetMathLibrary.BreakTransform` (`self.BattlePosition`)))
  (bind _unittarget (`self.UnitTarget`))
  ;[0 0 0 0.5] Use Technique on Enemy
  (`|AIMoveTo` (`self.UnitCharacter`) (0.0 0.0 0.0) (`self.UnitTarget`) 100.0
    (:`then`
      (bind _unitbattlehud (`self.UnitBattleHUD`)
        (:`then`
          (`/Game/Dynamic/Widgets/Battle/WBP_UnitBattleHUD.HideMenus` _unitbattlehud))
        (:`else`)))
    (:`OnSuccess`
      (`|SpawnActorFromClass` Technique (`Actor.GetTransform` _unittarget) "Undefined" "MultiplyWithRoot" null _unittarget (`self.UnitCharacter`))
      (`KismetSystemLibrary.Delay` 1.0)
      (`|AIMoveTo` (`self.UnitCharacter`) _battleposition_location null
        (:`then`
          (message `/Game/Dynamic/BlueprintInterfaces/BI_DynamicCamera.SetOrbit` (`Controller.GetViewTarget` (`GameplayStatics.GetPlayerController` 0)) false))
        (:`OnSuccess`
          (`self.RemoveUnitBattleHUD`)
          (`AIController.K2_SetFocus` (`AIBlueprintHelperLibrary.GetAIController` (`self.UnitCharacter`)) (`self.UnitTarget`))
          (`KismetSystemLibrary.Delay` 1.0)
          (`self.EndUnitTurn`))))))

(event `UseTechniqueOnAllies`
  (params (Technique :type "/Game/Dynamic/Abilities/Techniques/BP_TechniqueBase Class Reference"))
  (bind _unittarget (`self.UnitTarget`))
  (bind (_battleposition_location _battleposition_rotation) (`KismetMathLibrary.BreakTransform` (`self.BattlePosition`)))
  ;[0 0 0 0.5] Use Technique on Ally
  (`|AIMoveTo` (`self.UnitCharacter`) (`self.GetRangePosition` false) null 100.0
    (:`then`
      (`self.RemoveUnitBattleHUD`))
    (:`OnSuccess`
      (`|PlayMontage` (`Character.Mesh` (`self.UnitCharacter`)) (`self.ItemUseMontage`) (`self.ItemUsePlayRate`)
        (:`then`
          (message `/Game/Dynamic/BlueprintInterfaces/BI_DynamicCamera.SetLookAtActor` (`Controller.GetViewTarget` (`GameplayStatics.GetPlayerController` 0)) (`self.UnitTarget`))
          (message `/Game/Dynamic/BlueprintInterfaces/BI_DynamicCamera.SetDynamicLocation` (`Controller.GetViewTarget` (`GameplayStatics.GetPlayerController` 0)) (`self.UnitTarget`) (0.0 0.0 0.0)))
        (:`OnCompleted`
          (`|AIMoveTo` (`self.UnitCharacter`) _battleposition_location null
            (:`OnSuccess`
              (`AIController.K2_SetFocalPoint` (`AIBlueprintHelperLibrary.GetAIController` (`self.UnitCharacter`)) (+ _battleposition_location (* (`KismetMathLibrary.GetForwardVector` _battleposition_rotation) 200.0)))
              (`KismetSystemLibrary.Delay` 1.0)
              (`self.EndUnitTurn`))))
        (:`OnNotifyBegin`
          (`|SpawnActorFromClass` Technique (`Actor.GetTransform` _unittarget) "Undefined" "MultiplyWithRoot" null _unittarget (`self.UnitCharacter`)))))))

(event `RangedAttack`
  (bind _unitcharacter (`self.UnitCharacter`))
  (bind _unittarget (`self.UnitTarget`))
  ;[0 0 0 0.5] Basic Attack
  (`|AIMoveTo` (`self.UnitCharacter`) (`self.GetRangePosition` true) null 100.0
    (:`then`
      (`self.RemoveUnitBattleHUD`))
    (:`OnSuccess`
      (`|PlayMontage` (`Character.Mesh` (`self.UnitCharacter`)) (`self.AttackMontage`) (`self.AttackPlayRate`)
        (:`OnNotifyBegin`
          (bind _returnvalue (`|SpawnActorFromClass` (`self.ProjectalClass`) (`Actor.GetTransform` _unitcharacter) "Undefined" "MultiplyWithRoot" null _unitcharacter))
          (add `Actor.OnEndPlay` _returnvalue (delegate `EndRangedAttack`))
          (if (`KismetMathLibrary.ClassIsChildOf` (`GameplayStatics.GetObjectClass` (`self.UnitCharacter`)) "/Game/Dynamic/Characters/Battle/BP_PartyUnitBase.BP_PartyUnitBase_C")
            (message `/Game/Dynamic/BlueprintInterfaces/BI_DynamicCamera.SetDynamicLocation` (`Controller.GetViewTarget` (`GameplayStatics.GetPlayerController` 0)) null (`Actor.K2_GetActorLocation` (`self.UnitTarget`)))
            (else
              (message `/Game/Dynamic/BlueprintInterfaces/BI_DynamicCamera.SetDynamicLocation` (`Controller.GetViewTarget` (`GameplayStatics.GetPlayerController` 0)) _unittarget (`Actor.K2_GetActorLocation` _unittarget)))))))))

(event `EndRangedAttack`
  (params (Actor :type "Actor Object Reference") (EndPlayReason :type "EEndPlayReason Enum" :default "Destroyed"))
  (bind _battleposition_location (`KismetMathLibrary.BreakTransform` (`self.BattlePosition`)))
  ;[0 0 0 0.5] Basic Attack
  (`|AIMoveTo` (`self.UnitCharacter`) _battleposition_location null
    (:`then`
      (message `/Game/Dynamic/BlueprintInterfaces/BI_DynamicCamera.SetOrbit` (`Controller.GetViewTarget` (`GameplayStatics.GetPlayerController` 0)) false)
      (message `/Game/Dynamic/BlueprintInterfaces/BI_DynamicCamera.SetDynamicLocation` (`Controller.GetViewTarget` (`GameplayStatics.GetPlayerController` 0)) (`self.UnitCharacter`) (0.0 0.0 0.0)))
    (:`OnSuccess`
      (`AIController.K2_SetFocus` (`AIBlueprintHelperLibrary.GetAIController` (`self.UnitCharacter`)) (`self.UnitTarget`))
      (`KismetSystemLibrary.Delay` 1.0)
      (`self.EndUnitTurn`))))

(event `Cast Black Magic`
  (params (BlackMagicSpell :type "/Game/Dynamic/Abilities/Magic/BP_MagicBase Class Reference"))
  (bind _battleposition_location (`KismetMathLibrary.BreakTransform` (`self.BattlePosition`)))
  (bind _unittarget (`self.UnitTarget`))
  ;[0 0 0 0.5] Cast Magic
  ;;[0 0 0 0.5] Cast Black Magic
  (`|AIMoveTo` (`self.UnitCharacter`) (`self.GetRangePosition` true) null 100.0
    (:`then`
      (`self.RemoveUnitBattleHUD`))
    (:`OnSuccess`
      (`|PlayMontage` (`Character.Mesh` (`self.UnitCharacter`)) (`self.MagicCastMontage`) (`self.MagicCastPlayRate`)
        (:`then`
          (message `/Game/Dynamic/BlueprintInterfaces/BI_DynamicCamera.SetLookAtActor` (`Controller.GetViewTarget` (`GameplayStatics.GetPlayerController` 0)) (`self.UnitTarget`)))
        (:`OnCompleted`
          (`|AIMoveTo` (`self.UnitCharacter`) _battleposition_location null
            (:`OnSuccess`
              (`AIController.K2_SetFocus` (`AIBlueprintHelperLibrary.GetAIController` (`self.UnitCharacter`)) (`self.UnitTarget`))
              (`KismetSystemLibrary.Delay` 1.0)
              (`self.EndUnitTurn`))))
        (:`OnNotifyBegin`
          (`|SpawnActorFromClass` BlackMagicSpell (`Actor.GetTransform` _unittarget) "Undefined" "MultiplyWithRoot" null _unittarget (`self.UnitCharacter`)))))))

(event `CastWhiteMagic`
  (params (WhiteMagicSpell :type "/Game/Dynamic/Abilities/Magic/BP_MagicBase Class Reference"))
  (bind (_battleposition_location _battleposition_rotation) (`KismetMathLibrary.BreakTransform` (`self.BattlePosition`)))
  (bind _unittarget (`self.UnitTarget`))
  ;[0 0 0 0.5] Cast Magic
  ;;[0 0 0 0.5] Cast White Magic
  (`|AIMoveTo` (`self.UnitCharacter`) (`self.GetRangePosition` false) null 100.0
    (:`then`
      (`self.RemoveUnitBattleHUD`))
    (:`OnSuccess`
      (`|PlayMontage` (`Character.Mesh` (`self.UnitCharacter`)) (`self.MagicCastMontage`) (`self.MagicCastPlayRate`)
        (:`then`
          (message `/Game/Dynamic/BlueprintInterfaces/BI_DynamicCamera.SetLookAtActor` (`Controller.GetViewTarget` (`GameplayStatics.GetPlayerController` 0)) (`self.UnitTarget`))
          (message `/Game/Dynamic/BlueprintInterfaces/BI_DynamicCamera.SetDynamicLocation` (`Controller.GetViewTarget` (`GameplayStatics.GetPlayerController` 0)) (`self.UnitTarget`) (0.0 0.0 0.0)))
        (:`OnCompleted`
          (`|AIMoveTo` (`self.UnitCharacter`) _battleposition_location null
            (:`OnSuccess`
              (`AIController.K2_SetFocalPoint` (`AIBlueprintHelperLibrary.GetAIController` (`self.UnitCharacter`)) (+ _battleposition_location (* (`KismetMathLibrary.GetForwardVector` _battleposition_rotation) 200.0)))
              (`KismetSystemLibrary.Delay` 1.0)
              (`self.EndUnitTurn`))))
        (:`OnNotifyBegin`
          (`|SpawnActorFromClass` WhiteMagicSpell (`Actor.GetTransform` _unittarget) "Undefined" "MultiplyWithRoot" null _unittarget (`self.UnitCharacter`)))))))

(event `self.ReceiveTick`
  (params (DeltaSeconds :type "Float (single-precision)"))
  (bind _unitbattlehudwidget (`/Game/Dynamic/Characters/Battle/BP_UnitBase.UnitBattleHUDWidget` (`self.UnitCharacter`)))
  (bind (_returnvalue_roll _returnvalue_pitch _returnvalue_yaw) (`KismetMathLibrary.BreakRotator` (`KismetMathLibrary.FindLookAtRotation` (`SceneComponent.K2_GetComponentLocation` _unitbattlehudwidget) (`SceneComponent.K2_GetComponentLocation` (`PlayerCameraManager.TransformComponent` (`GameplayStatics.GetPlayerCameraManager` 0))))))
  ;[0 0 0 0.5] Event Tick
  (`SceneComponent.K2_SetWorldRotation` _unitbattlehudwidget (`KismetMathLibrary.MakeRotator` _returnvalue_roll _returnvalue_pitch _returnvalue_yaw) false false))

(fn `BeginBattle`
  (bind _returnvalue (`KismetSystemLibrary.K2_SetTimer` self "RequestTurn" (+ (* (- 1.0 (`KismetMathLibrary.NormalizeToRange` (* (`.AG_14_73FFEE6F4F6DA4E8F58BCFB2AA62EF48` (break `/Game/Dynamic/Data/S_StatTable` (`self.BaseUnitStats`))) (`.AG_22_73FFEE6F4F6DA4E8F58BCFB2AA62EF48` (break `/Game/Dynamic/Data/S_StatModifier` (`self.UnitStatModifier`)))) 0.0 99.0)) (- (`self.MaxActionTime`) (`self.MinActionTime`))) (`self.MinActionTime`))))
  (set `self.ActionTimer` _returnvalue))

(fn `CalculateBaseDamage`
  (returns (CalculatedDamage :type "Float (double-precision)"))
  (return (* (* (* (`.ST_11_50A9A38B4540B7AB4A52738E77ADB285` (break `/Game/Dynamic/Data/S_StatTable` (`self.BaseUnitStats`))) (`.ST_19_50A9A38B4540B7AB4A52738E77ADB285` (break `/Game/Dynamic/Data/S_StatModifier` (`self.UnitStatModifier`)))) 3.0) (`KismetMathLibrary.RandomFloatInRange` 0.9 1.1))))

(fn `CalculateDamage`
  (returns (BaseDamage :type "Float (double-precision)"))
  (bind _calculateddamage (`self.CalculateBaseDamage`))
  (return _calculateddamage))

(fn `CalculateDamageResistance`
  (params (BaseDamage :type "Float (double-precision)"))
  (returns (NewDamage :type "Float (double-precision)"))
  (return (/ (`KismetMathLibrary.MultiplyMultiply_FloatFloat` BaseDamage 2.0) (+ BaseDamage (* (`.EN_13_529D7A5A4A526EF885AFE3A64FB437D8` (break `/Game/Dynamic/Data/S_StatTable` (`self.BaseUnitStats`))) (`.EN_21_529D7A5A4A526EF885AFE3A64FB437D8` (break `/Game/Dynamic/Data/S_StatModifier` (`self.UnitStatModifier`))))))))

(fn `CalculateMagicBaseDamage`
  (params (SpellClass :type "/Game/Dynamic/Abilities/Magic/BP_MagicBase Class Reference"))
  (returns (`Magic Base Damage` :type "Float (double-precision)"))
  (bind (_abilityname _ablitydescription _rank _spelltarget _spellpowertable) (defaults `Object` (`local.SpellClass`)))
  (return (* (* (`.MG_12_F939C342436704CB530720A5A5F7A48E` (break `/Game/Dynamic/Data/S_StatTable` (`self.BaseUnitStats`))) (`.MG_20_F939C342436704CB530720A5A5F7A48E` (break `/Game/Dynamic/Data/S_StatModifier` (`self.UnitStatModifier`)))) (`KismetMathLibrary.Sqrt` (`BlueprintMapLibrary.Map_Find` _spellpowertable _rank)))))

(fn `EndUnitTurn`
  (`self.TurnEnded`)
  (`/Engine/EditorBlueprintResources/StandardMacros.IsValid` (`AIBlueprintHelperLibrary.GetAIController` (`self.UnitCharacter`))
    (:`Is Valid`
      (`self.BeginBattle`)
      (`AIController.K2_ClearFocus` (`AIBlueprintHelperLibrary.GetAIController` (`self.UnitCharacter`))))))

(fn `GetRangePosition`
  (params (TargettingEnemy :type Boolean))
  (returns (ReturnValue :type "Vector Structure"))
  (bind _unitcharacter (`self.UnitCharacter`))
  (bind _returnvalue (`Actor.K2_GetActorLocation` (`self.UnitCharacter`)))
  (return (`KismetMathLibrary.SelectVector` (+ _returnvalue (* (`KismetMathLibrary.GetDirectionUnitVector` _returnvalue (`Actor.K2_GetActorLocation` (`self.UnitTarget`))) 500.0)) (+ (`Actor.K2_GetActorLocation` _unitcharacter) (* (`Actor.GetActorForwardVector` _unitcharacter) 500.0)) TargettingEnemy)))

(fn `LevelUP`
  (`/Engine/EditorBlueprintResources/StandardMacros.IncrementInt` (`self.UnitLevel`)
    (:`  `
      (`self.LeveledUP`))))

(fn `RemoveUnitBattleHUD`
  (`|ExecutionSequence`
    (:`then_0`
      (bind _unitbattlehud (`self.UnitBattleHUD`)
        (:`then`
          (`WidgetComponent.SetWidget` (`/Game/Dynamic/Characters/Battle/BP_UnitBase.UnitBattleHUDWidget` (`self.UnitCharacter`)) null)
          (`Widget.RemoveFromParent` _unitbattlehud))
        (:`else`)))
    (:`then_1`
      (bind _infobarwidget (`self.InfoBarWidget`)
        (:`then`
          (`Widget.RemoveFromParent` _infobarwidget))
        (:`else`)))))

(fn `RequestTurn`
  (`/Engine/EditorBlueprintResources/StandardMacros.IsValid` (`AIBlueprintHelperLibrary.GetAIController` (`self.UnitCharacter`))
    (:`Is Valid`
      (bind _asgm_battle (cast `/Game/Dynamic/GameMode/GM_Battle` (`GameplayStatics.GetGameMode`)))
      (`/Game/Dynamic/GameMode/GM_Battle.TurnRequest` _asgm_battle (`self.UnitCharacter`)))))

(fn `RewardXP`
  (params (EXP :type Integer))
  (bind _exprequired (`self.EXPRequired`))
  (bind _output_get (set `self.EXPCurrent` (+ (`self.EXPCurrent`) EXP)))
  (if (> _output_get _exprequired)
    (`self.LevelUP`)
    (set `self.EXPCurrent` (mod _output_get _exprequired))))

(fn `SetCamera`
  (bind _returnvalue (`GameplayStatics.GetActorOfClass` "/Game/Dynamic/Blueprints/BP_DynamicCamera.BP_DynamicCamera_C"))
  (`PlayerController.SetViewTargetWithBlend` (`GameplayStatics.GetPlayerController` 0) _returnvalue 0.0 "VTBlend_Linear" 0.0 false)
  (message `/Game/Dynamic/BlueprintInterfaces/BI_DynamicCamera.SetDynamicLocation` _returnvalue (`self.UnitCharacter`) (0.0 0.0 0.0))
  (if (`KismetMathLibrary.ClassIsChildOf` (`GameplayStatics.GetObjectClass` (`self.UnitCharacter`)) "/Game/Dynamic/Characters/Battle/BP_PartyUnitBase.BP_PartyUnitBase_C")
    (message `/Game/Dynamic/BlueprintInterfaces/BI_DynamicCamera.SetRotation` (`Controller.GetViewTarget` (`GameplayStatics.GetPlayerController` 0)) (`self.UnitCharacter`))
    (else
      (message `/Game/Dynamic/BlueprintInterfaces/BI_DynamicCamera.SetOrbit` (`Controller.GetViewTarget` (`GameplayStatics.GetPlayerController` 0)) true))))

(fn `StartUnitTurn`
  (bind _unitcharacter (`self.UnitCharacter`))
  (`/Engine/EditorBlueprintResources/StandardMacros.IsValid` (`AIBlueprintHelperLibrary.GetAIController` (`self.UnitCharacter`))
    (:`Is Valid`
      (if (`KismetMathLibrary.ClassIsChildOf` (`GameplayStatics.GetObjectClass` (`self.UnitCharacter`)) "/Game/Dynamic/Characters/Battle/BP_PartyUnitBase.BP_PartyUnitBase_C")
        (bind _returnvalue (`|CreateWidget` "/Game/Dynamic/Widgets/Battle/WBP_InfoBar.WBP_InfoBar_C"))
        (bind _output_get (set `self.InfoBarWidget` _returnvalue))
        (`UserWidget.AddToViewport` _output_get 0)
        (bind _returnvalue_2 (`|CreateWidget` "/Game/Dynamic/Widgets/Battle/WBP_UnitBattleHUD.WBP_UnitBattleHUD_C" null _unitcharacter _output_get))
        (bind _output_get_2 (set `self.UnitBattleHUD` _returnvalue_2))
        (`WidgetComponent.SetWidget` (`/Game/Dynamic/Characters/Battle/BP_UnitBase.UnitBattleHUDWidget` _unitcharacter) _output_get_2)
        (`self.SetCamera`)
        (else
          ;[0 0 0 0.5] Enemy Action Select
          (bind _outactors (`GameplayStatics.GetAllActorsOfClass` "/Game/Dynamic/Characters/Battle/BP_PartyUnitBase.BP_PartyUnitBase_C"))
          (set `self.UnitTarget` (`KismetArrayLibrary.Array_Random` _outactors))
          (switch `int` (`KismetMathLibrary.RandomIntegerInRange` 0 2)
            (:`Default`
              _)
            (:`0`
              _)
            (:`1`
              _)
            (:`2`
              _))
          (`self.Attack Command`)
          (`self.SetCamera`))))
    (:`Is Not Valid`
      (`self.EndUnitTurn`))))