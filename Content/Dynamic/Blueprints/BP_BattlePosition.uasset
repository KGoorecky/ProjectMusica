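; BP_BattlePosition is a placement marker for a battle unit, flagged as either an enemy or non-enemy position.
; The construction script colors its arrow red for enemy placements and blue otherwise.
; On BeginPlay only non-enemy positions call SpawnUnit, which spawns a valid UnitClass at the marker's transform, adjusting for collisions but always spawning.
; Enemy positions do not spawn anything on their own.
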(event `self.ReceiveBeginPlay`
  (if (not (`self.IsEnemyPlacement`))
    (`self.SpawnUnit`)))

(fn `SpawnUnit`
  (bind _unitclass (`self.UnitClass`)
    (:`then`
      (`|SpawnActorFromClass` _unitclass (`self.GetTransform`) "AdjustIfPossibleButAlwaysSpawn" "MultiplyWithRoot" null null))
    (:`else`)))

(fn `UserConstructionScript`
  (`ArrowComponent.SetArrowColor` (`self.Arrow`) (`KismetMathLibrary.SelectColor` (struct :`R` 1.0 :`A` 1.0) (struct :`B` 1.0 :`A` 1.0) (`self.IsEnemyPlacement`))))