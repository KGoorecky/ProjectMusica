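; BP_DynamicCamera is a battle camera actor that frames party units, orbits, follows actors or looks at targets.
; Set events reconfigure the spring arm, rotating movement and attachment, or store a target location and rotation.
; While it has no attach parent, Tick interpolates the actor location and camera rotation toward those targets.
; Tick also starts a battle camera shake every frame while the party-unit flag from SetRotation is set.
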(event `CameraShake`
  (if (`self.IsOnPartyUnit`)
    (`PlayerController.ClientStartCameraShake` :`self` (`GameplayStatics.GetPlayerController` 0) :`Shake` "/Game/Dynamic/Blueprints/CS_BattleShake.CS_BattleShake_C")))

(event `self.ReceiveTick`
  (params (DeltaSeconds :type "Float (single-precision)"))
  ;[0 0 0 0.5] Event Tick
  (`self.CameraShake`)
  (`/Engine/EditorBlueprintResources/StandardMacros.IsValid` (`self.GetAttachParentActor`)
    (:`Is Not Valid`
      (`self.K2_SetActorLocation` (`KismetMathLibrary.VInterpTo` (`self.K2_GetActorLocation`) (`self.TargetLocation`) (`GameplayStatics.GetWorldDeltaSeconds`) 5.0))
      (`SceneComponent.K2_SetWorldRotation` (`self.Camera`) (`KismetMathLibrary.RInterpTo` (`SceneComponent.K2_GetComponentRotation` (`self.Camera`)) (`self.TargetRotation`) (`GameplayStatics.GetWorldDeltaSeconds`) 5.0) false false))))

(event `/Game/Dynamic/BlueprintInterfaces/BI_DynamicCamera.SetRotation`
  (params (Actor :type "Actor Object Reference"))
  ;[0 0 0 0.5] Set Rotation (for Camera behind Character)
  (`SceneComponent.K2_SetRelativeRotation` (`self.SpringArm`) (`KismetMathLibrary.MakeRotator` (.roll (`self.K2_GetActorRotation` Actor)) (+ (.pitch (`self.K2_GetActorRotation` Actor)) -15.0) (+ (.yaw (`self.K2_GetActorRotation` Actor)) -20.0)) false false)
  (set `SpringArmComponent.TargetArmLength` 256.0 (`self.SpringArm`))
  (set `RotatingMovementComponent.RotationRate` (struct) (`self.RotatingMovement`))
  (set `SpringArmComponent.SocketOffset` (0.0 128.0 0.0) (`self.SpringArm`))
  (set `self.IsOnPartyUnit` true))

(event `/Game/Dynamic/BlueprintInterfaces/BI_DynamicCamera.SetOrbit`
  (params (IsOrbiting :type Boolean))
  ;[0 0 0 0.5] Set Orbit
  (set `RotatingMovementComponent.RotationRate` (`KismetMathLibrary.SelectRotator` (struct :`Yaw` 10.0) (struct) IsOrbiting) (`self.RotatingMovement`))
  (`SceneComponent.K2_SetRelativeRotation` (`self.SpringArm`) (struct :`Pitch` -30.0) false false)
  (set `SpringArmComponent.TargetArmLength` 512.0 (`self.SpringArm`))
  (bind _output_get (set `SpringArmComponent.bInheritYaw` IsOrbiting (`self.SpringArm`)))
  (if (not _output_get)
    (`self.K2_SetActorRotation` (struct)))
  (set `SpringArmComponent.SocketOffset` (0.0 0.0 0.0) (`self.SpringArm`))
  (set `self.IsOnPartyUnit` false))

(event `/Game/Dynamic/BlueprintInterfaces/BI_DynamicCamera.SetDynamicLocation`
  (params (Actor :type "Actor Object Reference") (Vector :type "Vector Structure"))
  ;[0 0 0 0.5] Set Dynamic Location
  (`/Engine/EditorBlueprintResources/StandardMacros.IsValid` Actor
    (:`Is Valid`
      (`self.K2_AttachToActor` Actor "None" "SnapToTarget" "KeepWorld" "KeepWorld")
      (`SceneComponent.K2_SetRelativeRotation` :`self` (`self.Camera`))
      (set `self.TargetLocation` (`self.K2_GetActorLocation` Actor)))
    (:`Is Not Valid`
      (bind _output_get (set `self.TargetLocation` Vector))
      (`self.K2_DetachFromActor` "KeepWorld" "KeepWorld" "KeepWorld")
      (bind (_returnvalue_roll _returnvalue_pitch _returnvalue_yaw) (`KismetMathLibrary.BreakRotator` (`KismetMathLibrary.FindLookAtRotation` (`SceneComponent.K2_GetComponentLocation` (`self.Camera`)) _output_get)))
      (set `self.TargetRotation` (`KismetMathLibrary.MakeRotator` (+ _returnvalue_roll 15.0) (+ _returnvalue_pitch -20.0) _returnvalue_yaw))))
  (set `self.IsOnPartyUnit` false))

(event `/Game/Dynamic/BlueprintInterfaces/BI_DynamicCamera.SetLookAtActor`
  (params (TargetActor :type "Actor Object Reference"))
  ;[0 0 0 0.5] Set Look at Actor
  (set `self.TargetRotation` (`KismetMathLibrary.FindLookAtRotation` (`PlayerCameraManager.GetCameraLocation` (`GameplayStatics.GetPlayerCameraManager` 0)) (`self.K2_GetActorLocation` TargetActor)))
  (`self.K2_DetachFromActor` "KeepWorld" "KeepWorld" "KeepWorld")
  (set `self.IsOnPartyUnit` false))

(fn `UserConstructionScript`)