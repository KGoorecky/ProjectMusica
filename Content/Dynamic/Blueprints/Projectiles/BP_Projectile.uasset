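; Base projectile fired by units, delivering combat damage and impact effects when it hits.
; It ignores its instigator while moving and spawns a Niagara impact at the hit actor's location.
; Damage comes from the instigating BP_UnitBase's CombatComponent and goes to that component's UnitTarget, not necessarily the actor struck.
; It then plays a sound, removes its Niagara trail component and destroys itself after a short delay.
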(event `self.ReceiveBeginPlay`
  ;[0 0 0 0.5] BeginPlay
  (`PrimitiveComponent.IgnoreActorWhenMoving` (`self.SphereCollision`) (`self.GetInstigator`) true))

(event `self.ReceiveHit`
  (params (MyComp :type "PrimitiveComponent Object Reference") (Other :type "Actor Object Reference") (OtherComp :type "PrimitiveComponent Object Reference") (bSelfMoved :type Boolean) (HitLocation :type "Vector Structure") (HitNormal :type "Vector Structure") (NormalImpulse :type "Vector Structure") (Hit :type "HitResult Structure (by ref)"))
  ;[0 0 0 0.5] Event Hit
  (`NiagaraFunctionLibrary.SpawnSystemAtLocation` (`self.ImpactEffect`) (`self.K2_GetActorLocation` Other))
  (bind _asbp_unit_base (cast `/Game/Dynamic/Characters/Battle/BP_UnitBase` (`self.GetInstigator`)))
  (bind _combat_component (`/Game/Dynamic/Characters/Battle/BP_UnitBase.Combat Component` _asbp_unit_base))
  (bind _basedamage (`/Game/Dynamic/Blueprints/Components/AC_Combat.CalculateDamage` _combat_component))
  (`GameplayStatics.ApplyDamage` (`/Game/Dynamic/Blueprints/Components/AC_Combat.UnitTarget` _combat_component) _basedamage null _asbp_unit_base (`self.Damage Type Class`))
  (`GameplayStatics.PlaySoundAtLocation` (`self.ProjectileSoundEffect`) (`self.K2_GetActorLocation`) (struct) 1.0 1.0 0.0 null null null null)
  (`ActorComponent.K2_DestroyComponent` (`self.NiagaraSystem`))
  (`KismetSystemLibrary.Delay` 1.0)
  (`self.K2_DestroyActor`))

(fn `UserConstructionScript`)