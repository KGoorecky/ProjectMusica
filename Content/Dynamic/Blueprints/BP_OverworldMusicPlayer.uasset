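; BP_OverworldMusicPlayer plays the overworld MetaSound music and switches it between normal and enemy-spotted versions.
; On BeginPlay it assigns the MetaSound to its music player component and starts playback.
; ChangeMusicType checks the FocusedEnemies array and sends the matching trigger parameter to the MetaSound.
; A DoOnce keeps the spotted trigger from refiring until the array is found empty, which resets it.
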(event `self.ReceiveBeginPlay`
  (`AudioComponent.SetSound` (`self.MusicPlayerComponent`) (`self.MetaSoundMusic`))
  (`AudioComponent.Play` (`self.MusicPlayerComponent`) 0.0))

(fn `ChangeMusicType`
  (if (> (`KismetArrayLibrary.Array_Length` (`self.FocusedEnemies`)) 0)
    (`/Engine/EditorBlueprintResources/StandardMacros.DoOnce` false :!label _label
      (:`Completed`
        (`AudioParameterControllerInterface.SetTriggerParameter` (`self.MusicPlayerComponent`) "ChangeMusicToSpottedVersion")))
    (else
      (`AudioParameterControllerInterface.SetTriggerParameter` (`self.MusicPlayerComponent`) "ChangeMusicToNormalVersion")
      (goto _label :!via `Reset`))))

(fn `UserConstructionScript`)