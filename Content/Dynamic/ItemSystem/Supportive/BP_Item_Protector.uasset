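; Supportive item Blueprint for the Protector, a timed buff that raises the EN stat of its recipient.
; On BeginPlay it runs the parent logic, adds a flat bonus to EN in the recipient CombatComponent's UnitStatModifier and starts a 30-second timer.
; When the timer fires, ItemDropOff subtracts the same bonus, and the Niagara component destroys itself when its system finishes.
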(event `self.ReceiveBeginPlay`
  (bind _unitstatmodifier (`/Game/Dynamic/Blueprints/Components/AC_Combat.UnitStatModifier` (`/Game/Dynamic/Characters/Battle/BP_UnitBase.Combat Component` (`self.Recipient`))))
  (`parent.ReceiveBeginPlay`)
  (setmembers `/Game/Dynamic/Data/S_StatModifier` :`StructRef` _unitstatmodifier :`EN` (+ (`.EN_21_529D7A5A4A526EF885AFE3A64FB437D8` (break `/Game/Dynamic/Data/S_StatModifier` _unitstatmodifier)) 1.0))
  (`KismetSystemLibrary.K2_SetTimerDelegate` (delegate `ItemDropOff`) 30.0))

(event `self.Niagara.OnSystemFinished`
  (params (PSystem :type "NiagaraComponent Object Reference"))
  (`ActorComponent.K2_DestroyComponent` PSystem))

(event `ItemDropOff`
  (bind _unitstatmodifier (`/Game/Dynamic/Blueprints/Components/AC_Combat.UnitStatModifier` (`/Game/Dynamic/Characters/Battle/BP_UnitBase.Combat Component` (`self.Recipient`))))
  (setmembers `/Game/Dynamic/Data/S_StatModifier` :`StructRef` _unitstatmodifier :`EN` (- (`.EN_21_529D7A5A4A526EF885AFE3A64FB437D8` (break `/Game/Dynamic/Data/S_StatModifier` _unitstatmodifier)) 1.0)))

(fn `UserConstructionScript`
  (`parent.UserConstructionScript`))